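; Base projectile actor that flies by projectile movement, ignores its owner and reports impacts through an OnProjectileImpact dispatcher.
; The construction script applies speed and gravity and enables homing when flagged with a valid Target.
; On BeginPlay, a valid Target sets initial velocity toward it and starts a short self-destruct delay; untargeted projectiles get no such timeout.
; Blocking hits broadcast the impact, play effect and sound, then destroy the actor.
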(event OnComponentHit(BoxCollision)
  (params (HitComponent :type Primitive%20Component%20Object%20Reference) (OtherActor :type Actor%20Object%20Reference) (OtherComp :type Primitive%20Component%20Object%20Reference) (NormalImpulse :type Vector :default "0, 0, 0") (Hit :type Hit%20Result%20Structure%20%28by%20ref%29))
  (bind _location (Collision|BreakHitResult Hit))
  (Default|CallOnProjectileImpact OtherActor Hit)
  (Effects|SpawnEmitteratLocation (Variables|Effects|GetImpact%20Effect) _location "0, 0, 0" (Variables|Default|GetScale))
  (Audio|PlaySoundatLocation (Variables|Sounds|GetImpact%20Sound) _location "0, 0, 0" 1.0 1.0 0.0 0 0 0 0)
  (Actor|DestroyActor))

(event OnComponentBeginOverlap(BoxCollision)
  (params (OverlappedComponent :type Primitive%20Component%20Object%20Reference) (OtherActor :type Actor%20Object%20Reference) (OtherComp :type Primitive%20Component%20Object%20Reference) (OtherBodyIndex :type Integer) (bFromSweep :type Boolean) (SweepResult :type Hit%20Result%20Structure%20%28by%20ref%29)))

(event Custom|RotateToTarget
  (Variables|/Script/Engine.MovementComponent|SetVelocity (Variables|Default|GetProjectileMovement) (* (Math|Vector|GetUnitDirection(Vector) (Transformation|GetActorLocation) (Transformation|GetActorLocation (Variables|Target|GetTarget))) (Variables|ProjectileSettings|GetSpeed))))

(event EventBeginPlay
  (Collision|IgnoreActorwhenMoving (Variables|Default|GetBox%20Collision) (Components|GetOwner) true)
  (Variables|Target|GetTarget
    (:then
      (CallFunction|RotatetoTarget)
      (Utilities|FlowControl|Delay 2.0)
      (Actor|DestroyActor))
    (:else)))

(fn ConstructionScript
  (bind _projectilemovement (Variables|Default|GetProjectileMovement))
  (bind _projectilemovement_2 (Variables|Default|GetProjectileMovement))
  (Variables|/Script/Engine.ProjectileMovementComponent|SetInitialSpeed _projectilemovement (Variables|ProjectileSettings|GetSpeed))
  (Variables|/Script/Engine.ProjectileMovementComponent|SetMaxSpeed _projectilemovement (Variables|ProjectileSettings|GetSpeed))
  (Variables|/Script/Engine.ProjectileMovementComponent|SetProjectileGravityScale _projectilemovement (Variables|ProjectileSettings|GetGravity))
  (Variables|Target|GetTarget
    (:then
      (if (Variables|ProjectileSettings|GetisHoming)
        (Variables|/Script/Engine.ProjectileMovementComponent|SetbIsHomingProjectile _projectilemovement_2 true)
        (Variables|/Script/Engine.ProjectileMovementComponent|SetHomingTargetComponent _projectilemovement_2 (Variables|/Script/Engine.Actor|GetRootComponent (Variables|Target|GetTarget)))))
    (:else)))