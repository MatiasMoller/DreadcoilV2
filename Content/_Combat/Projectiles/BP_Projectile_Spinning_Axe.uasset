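; Spinning axe projectile that briefly ignores pawns after spawning while its mesh spins in flight.
; On BeginPlay it runs the parent's logic, sets the box collision to ignore the Pawn channel, then restores blocking after a short delay.
; A timeline drives the mesh's world yaw, keeping pitch and roll, and restarts itself on finish to spin continuously.
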(event Custom|SpinAxe
  (bind _mesh (Variables|Character|GetMesh))
  (bind _returnvalue (Transformation|GetWorldRotation _mesh))
  (bind _z_rotation (Timeline|RotationTimeline PlayFromStart)
    (:Update
      (Transformation|SetWorldRotation _mesh (Math|Rotator|MakeRotator (.roll _returnvalue) (.pitch _returnvalue) _z_rotation) false false))
    (:Finished
      (CallFunction|SpinAxe))))

(event EventBeginPlay
  (|CallParentFunction)
  (Collision|SetCollisionResponsetoChannel (Variables|Default|GetBox%20Collision) "ECC_Pawn" "ECR_Ignore")
  (CallFunction|SpinAxe)
  (Utilities|FlowControl|Delay 0.2)
  (Collision|SetCollisionResponsetoChannel (Variables|Default|GetBox%20Collision) "ECC_Pawn" "ECR_Block"))

(event Collision|EventActorBeginOverlap
  (params (OtherActor :type Actor%20Object%20Reference)))

(event EventTick
  (params (DeltaSeconds :type Float%20%28single-precision%29)))

(fn ConstructionScript
  (|CallParentFunction))