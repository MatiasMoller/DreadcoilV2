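; BP_RowOfTorches is an environment actor that lights a row of fire effects in sequence when the player enters a trigger.
; Overlapping Box or Box1 activates the first pair of NewFire components, a second pair after a delay, then the rest individually at shorter intervals.
; Box activates without resetting, while Box1 passes the reset flag to every fire except NewFire3.
; Neither trigger deactivates the fires.
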(event OnComponentBeginOverlap(Box)
  (params (OverlappedComponent :type Primitive%20Component%20Object%20Reference) (OtherActor :type Actor%20Object%20Reference) (OtherComp :type Primitive%20Component%20Object%20Reference) (OtherBodyIndex :type Integer) (bFromSweep :type Boolean) (SweepResult :type Hit%20Result%20Structure%20%28by%20ref%29))
  (if (== OtherActor (Game|GetPlayerCharacter 0))
    (Components|Activation|Activate (Variables|Default|GetNewFire) false)
    (Components|Activation|Activate (Variables|Default|GetNewFire1) false)
    (Utilities|FlowControl|Delay 1.0)
    (Components|Activation|Activate (Variables|Default|GetNewFire3) false)
    (Components|Activation|Activate (Variables|Default|GetNewFire2) false)
    (Utilities|FlowControl|Delay 0.5)
    (Components|Activation|Activate (Variables|Default|GetNewFire4) false)
    (Utilities|FlowControl|Delay 0.5)
    (Components|Activation|Activate (Variables|Default|GetNewFire5) false)
    (Utilities|FlowControl|Delay 0.5)
    (Components|Activation|Activate (Variables|Default|GetNewFire6) false)
    (Utilities|FlowControl|Delay 0.5)
    (Components|Activation|Activate (Variables|Default|GetNewFire7) false)
    (Utilities|FlowControl|Delay 0.5)
    (Components|Activation|Activate (Variables|Default|GetNewFire8) false)))

(event OnComponentBeginOverlap(Box1)
  (params (OverlappedComponent :type Primitive%20Component%20Object%20Reference) (OtherActor :type Actor%20Object%20Reference) (OtherComp :type Primitive%20Component%20Object%20Reference) (OtherBodyIndex :type Integer) (bFromSweep :type Boolean) (SweepResult :type Hit%20Result%20Structure%20%28by%20ref%29))
  (if (== OtherActor (Game|GetPlayerCharacter 0))
    (Components|Activation|Activate (Variables|Default|GetNewFire) true)
    (Components|Activation|Activate (Variables|Default|GetNewFire1) true)
    (Utilities|FlowControl|Delay 1.0)
    (Components|Activation|Activate (Variables|Default|GetNewFire3) false)
    (Components|Activation|Activate (Variables|Default|GetNewFire2) true)
    (Utilities|FlowControl|Delay 0.5)
    (Components|Activation|Activate (Variables|Default|GetNewFire4) true)
    (Utilities|FlowControl|Delay 0.5)
    (Components|Activation|Activate (Variables|Default|GetNewFire5) true)
    (Utilities|FlowControl|Delay 0.5)
    (Components|Activation|Activate (Variables|Default|GetNewFire6) true)
    (Utilities|FlowControl|Delay 0.5)
    (Components|Activation|Activate (Variables|Default|GetNewFire7) true)
    (Utilities|FlowControl|Delay 0.5)
    (Components|Activation|Activate (Variables|Default|GetNewFire8) true)))

(fn ConstructionScript)