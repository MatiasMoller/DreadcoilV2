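; Interactable bonfire that refills the player's healing flasks and serves as a checkpoint.
; The first Interact activates its fire particles and looping cue; every use plays the player animation, sound and light flare, then refills flasks after a delay.
; Timelines fade the light back down, and a DoOnce blocks reuse until the fade ends, resetting only if the player animation has finished.
; Separate overlap volumes toggle the prompt widget and register the checkpoint.
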(event OnComponentBeginOverlap(Box)
  (params (OverlappedComponent :type Primitive%20Component%20Object%20Reference) (OtherActor :type Actor%20Object%20Reference) (OtherComp :type Primitive%20Component%20Object%20Reference) (OtherBodyIndex :type Integer) (bFromSweep :type Boolean) (SweepResult :type Hit%20Result%20Structure%20%28by%20ref%29))
  (Utilities|Casting|CastToBP_Player OtherActor)
  (Rendering|SetVisibility (Variables|Default|GetWidget) true false))

(event OnComponentEndOverlap(Box)
  (params (OverlappedComponent :type Primitive%20Component%20Object%20Reference) (OtherActor :type Actor%20Object%20Reference) (OtherComp :type Primitive%20Component%20Object%20Reference) (OtherBodyIndex :type Integer))
  (Utilities|Casting|CastToBP_Player OtherActor)
  (Rendering|SetVisibility (Variables|Default|GetWidget) false false))

(event OnComponentBeginOverlap(CheckpointCollision)
  (params (OverlappedComponent :type Primitive%20Component%20Object%20Reference) (OtherActor :type Actor%20Object%20Reference) (OtherComp :type Primitive%20Component%20Object%20Reference) (OtherBodyIndex :type Integer) (bFromSweep :type Boolean) (SweepResult :type Hit%20Result%20Structure%20%28by%20ref%29))
  ;[1 1 1] Add Checkpoint
  (if (== OtherActor (Game|GetPlayerCharacter 0))
    (Class|BPIInteract|SetCurrentCheckpoint(Message) OtherActor self)))

(event EventBeginPlay
  (bind _asbp_player (Utilities|Casting|CastToBP_Player (Game|GetPlayerCharacter 0)))
  (Variables|Default|SetAs%20BP%20Player _asbp_player))

(event Collision|EventActorBeginOverlap
  (params (OtherActor :type Actor%20Object%20Reference)))

(event EventTick
  (params (DeltaSeconds :type Float%20%28single-precision%29)))

(event EventInteract
  (bind _as_bp_player (Variables|Default|GetAs%20BP%20Player))
  (bind _as_bp_player_2 (Variables|Default|GetAs%20BP%20Player))
  (bind _bpc_damagesystem (Variables|/Game/_Player/BP_Player.BP_Player_C|GetBPC_DamageSystem _as_bp_player_2))
  (bind _bpc_damagesystem_2 (Variables|/Game/_Player/BP_Player.BP_Player_C|GetBPC_DamageSystem _as_bp_player))
  (Utilities|FlowControl|DoOnce false :!label _label
    (:Completed
      (if (Variables|Default|GetActivated)
        (Default|BonfireAnim (Variables|Default|GetAs%20BP%20Player))
        (Audio|PlaySoundatLocation "/Game/_SFX/Bonfire_lit_2.Bonfire_lit_2" (Transformation|GetActorLocation) "0, 0, 0" 1.0 1.0 0.0 0 0 0 0)
        (Rendering|Components|Light|SetIntensity (Variables|Default|GetPointLight) 3e+04)
        (Utilities|FlowControl|Delay 2.0)
        (Variables|/Game/_Combat/BPC_DamageSystem.BPC_DamageSystem_C|SetCurrentFlasks _bpc_damagesystem (Variables|/Game/_Combat/BPC_DamageSystem.BPC_DamageSystem_C|GetMaxFlasks _bpc_damagesystem))
        (bind _newtrack_0 (Timeline|Timeline PlayFromStart)
          (:Update
            (Rendering|Components|Light|SetIntensity (Variables|Default|GetPointLight) (Math|Float|Lerp 3e+04 5e+03 _newtrack_0)))
          (:Finished
            (if (Variables|/Game/_Player/BP_Player.BP_Player_C|GetHas%20animation%20Finished? (Variables|Default|GetAs%20BP%20Player))
              (goto _label Reset))))
        (else
          (Variables|Default|SetActivated true)
          (Components|Activation|Activate (Variables|Default|GetBonfire_constant_Cue) false)
          (Default|BonfireAnim (Variables|Default|GetAs%20BP%20Player))
          (Components|Activation|Activate (Variables|Default|GetParticleSystem) false)
          (Audio|PlaySoundatLocation "/Game/_SFX/Bonfire_lit_2.Bonfire_lit_2" (Transformation|GetActorLocation) "0, 0, 0" 1.0 1.0 0.0 0 0 0 0)
          (Rendering|Components|Light|SetIntensity (Variables|Default|GetPointLight) 3e+04)
          (Utilities|FlowControl|Delay 2.0)
          (Variables|/Game/_Combat/BPC_DamageSystem.BPC_DamageSystem_C|SetCurrentFlasks _bpc_damagesystem_2 (Variables|/Game/_Combat/BPC_DamageSystem.BPC_DamageSystem_C|GetMaxFlasks _bpc_damagesystem_2))
          (bind _newtrack_0_2 (Timeline|BonfireFadeOut PlayFromStart)
            (:Update
              (Rendering|Components|Light|SetIntensity (Variables|Default|GetPointLight) (Math|Float|Lerp 3e+04 5e+03 _newtrack_0_2)))
            (:Finished
              (if (Variables|/Game/_Player/BP_Player.BP_Player_C|GetHas%20animation%20Finished? (Variables|Default|GetAs%20BP%20Player))
                (goto _label Reset)))))))))

(fn ConstructionScript)