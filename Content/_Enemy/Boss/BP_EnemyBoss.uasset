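; Boss enemy that extends a parent enemy with an attached axe, dedicated health bar and roaring intro.
; Attacks run through BPCAttacks or montage notifies, spanning melee combos, slams, homing axe throws and lightning.
; Teleport fakes a blink via invisible high-speed flying AIMoveTo; floating uses a spawned platform with invincibility, both signalling completion through dispatchers.
; Death stops AI, returns attack tokens, ragdolls, then shows boss-defeated and paused game-over screens.
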(event Custom|EquipWeapon
  ;[1 1 1] Equip/Unequip Axe
  (bind _returnvalue (Game|SpawnActorfromClass "/Game/_Enemy/Boss/Axe/BP_Axe.BP_Axe_C" (Math|Transform|MakeTransform "0, 0, 0" "0, 0, 0" "1.000000,1.000000,1.000000") "Undefined" "MultiplyWithRoot" 0 0))
  (bind _output_get (Variables|Default|SetAxe%20Ref _returnvalue))
  (Transformation|AttachComponentToComponent _output_get (Variables|Character|GetMesh) "AxeSocket" "SnapToTarget" "SnapToTarget" "SnapToTarget" true))

(event Custom|UnequipWeapon
  ;[1 1 1] Equip/Unequip Axe
  (bind _axe_ref (Variables|Default|GetAxe%20Ref)
    (:then
      (Actor|DestroyActor _axe_ref))
    (:else)))

(event Custom|Ground%20Smash
  (params (Attack%20Target :type Actor%20Object%20Reference))
  ;[1 0 0] ATTACKS
  (Default|GroundSmash (Variables|Default|GetBPC_Attacks) (Utilities|Struct|MakeS_AttackInfo Attack%20Target "/Game/_Enemy/Boss/NewAnimations/Attacks/AxeGroundSlam_UE_Montage.AxeGroundSlam_UE_Montage" (Utilities|Struct|MakeS_DamageInfo 3e+01 "NewEnumerator3" "NewEnumerator1" false false false true)) 1.1e+03))

(event Custom|StartFloat
  (bind _returnvalue (Transformation|GetActorLocation))
  ;[1 1 1] Floating Base
  (Utilities|FlowControl|DoOnce false
    (:Completed
      (Variables|/Game/_Combat/BPC_DamageSystem.BPC_DamageSystem_C|SetisInvincible (Variables|Default|GetBPC_DamageSystem) true)
      (bind _outhit (Collision|LineTraceByChannel _returnvalue (* _returnvalue "0.000000,0.000000,1000.000000") "TraceTypeQuery1" false 0 "None"))
      (bind _returnvalue_2 (Game|SpawnActorfromClass "/Game/_Props/BP_FloatingPlatform.BP_FloatingPlatform_C" (Math|Transform|MakeTransform (.Location (Collision|BreakHitResult _outhit)) "0, 0, 0" "1.000000,1.000000,1.000000") "Undefined" "MultiplyWithRoot" 0 0))
      (bind _output_get (Variables|Default|SetFloatingPlatformREF _returnvalue_2))
      (EventDispatchers|AssignOnFloatTimelineFinish _output_get (delegate Custom|OnFloatTimelineFinish_Event)))))

(event Custom|OnFloatTimelineFinish_Event
  ;[1 1 1] Floating Base
  (EventDispatchers|UnbindEventfromOnFloatTimelineFinish (stale Custom|StartFloat _output_get) (delegate Custom|OnFloatTimelineFinish_Event))
  (Default|CallOnFloatHeightReached))

(event Custom|AOETrail
  (params (Attack%20Target :type Actor%20Object%20Reference))
  ;[1 0 0] ATTACKS
  (CallFunction|Attack Attack%20Target)
  (bind _notifyname (Animation|Montage|PlayMontage (Variables|Character|GetMesh) "/Game/_Enemy/Boss/NewAnimations/Attacks/Battlecry_UE_Montage.Battlecry_UE_Montage")
    (:OnCompleted
      (CallFunction|AttackEnd Attack%20Target :!label _label))
    (:OnInterrupted
      (goto _label))
    (:OnNotifyBegin
      (switch name _notifyname
        (:Strike
          (bind _returnvalue (Game|SpawnActorfromClass "/Game/_Combat/AOE/BP_BossLightning.BP_BossLightning_C" (Math|Transform|MakeTransform "0, 0, 0" "0, 0, 0" "1.000000,1.000000,1.000000") "Undefined" "MultiplyWithRoot" 0 0.5 Attack%20Target "/Game/FXVarietyPack/Particles/Boss_Lightning.Boss_Lightning" false false false 0))
          (EventDispatchers|AssignOnAOEOverlappedActor _returnvalue (delegate Custom|OnAOEOverlappedActor_Event)))))))

(event Custom|OnFloatTimelineFinish_Event_0
  ;[1 1 1] Floating Base
  (EventDispatchers|UnbindEventfromOnFloatTimelineFinish (stale Custom|StopFloat _floatingplatformref) (delegate Custom|OnFloatTimelineFinish_Event_0))
  (Actor|DestroyActor (stale Custom|StopFloat _floatingplatformref))
  (Variables|/Game/_Combat/BPC_DamageSystem.BPC_DamageSystem_C|SetisInvincible (Variables|Default|GetBPC_DamageSystem) false)
  (Default|CallOnFloatEnded))

(event Custom|StopFloat
  (bind _returnvalue (Transformation|GetActorLocation))
  ;[1 1 1] Floating Base
  (Utilities|FlowControl|Sequence
    (:then_0
      (bind _floatingplatformref (Variables|Default|GetFloatingPlatformREF)
        (:then
          _)
        (:else
          _))
      (Default|StopFloating _floatingplatformref)
      (EventDispatchers|AssignOnFloatTimelineFinish _floatingplatformref (delegate Custom|OnFloatTimelineFinish_Event_0)))
    (:then_1
      (Utilities|FlowControl|DoOnce false) ; enters at Reset
    )))

(event Custom|OnAOEOverlappedActor_Event
  (params (Actor :type Actor%20Object%20Reference))
  ;[1 0 0] ATTACKS
  (Class|BPIDamagable|TakeDamage(Message) Actor (Utilities|Struct|MakeS_DamageInfo 3e+01 "NewEnumerator3" "NewEnumerator1") self))

(event Custom|Intro
  (bind _bpc_damagesystem (Variables|Default|GetBPC_DamageSystem))
  (Utilities|FlowControl|DoOnce false
    (:Completed
      (Variables|Default|SetHasIntroFinished false)
      (Variables|/Game/_Combat/BPC_DamageSystem.BPC_DamageSystem_C|SetisInvincible _bpc_damagesystem true)
      (Animation|Montage|PlayMontage (Variables|Character|GetMesh) "/Game/_Enemy/Boss/NewAnimations/MutantRoaring_UE_Montage.MutantRoaring_UE_Montage" 1.5
        (:OnCompleted
          (Variables|/Game/_Combat/BPC_DamageSystem.BPC_DamageSystem_C|SetisInvincible _bpc_damagesystem false)
          (Variables|Default|SetHasIntroFinished true)
          (Default|CallOnIntroFinish))))))

(event Custom|AttackCombo1
  (params (AttackTarget :type Actor%20Object%20Reference))
  ;[1 0 0] ATTACKS
  (Default|PrimaryMeleeAttack (Variables|Default|GetBPC_Attacks) (Utilities|Struct|MakeS_AttackInfo AttackTarget "/Game/_Enemy/Boss/NewAnimations/Attacks/BossThreeSwingCombo_UE_Montage.BossThreeSwingCombo_UE_Montage" (Utilities|Struct|MakeS_DamageInfo 2e+01 "NewEnumerator1" "NewEnumerator1" false true true)) 4e+01 2.2e+02))

(event Custom|Teleport
  (params (Location :type Vector) (AttackTarget :type Actor%20Object%20Reference))
  (bind _charactermovement (Variables|Character|GetCharacterMovement))
  ;[0 0.3458 1] Teleport
  (if (not (Variables|Default|GetisTeleporting))
    (Variables|Default|SetisTeleporting true)
    (Pawn|Components|CharacterMovement|SetMovementMode _charactermovement "MOVE_Flying" 0)
    (Variables|/Script/Engine.CharacterMovementComponent|SetMaxFlySpeed _charactermovement 5e+03)
    (Variables|/Script/Engine.CharacterMovementComponent|SetMaxAcceleration _charactermovement 99999.0)
    (Rendering|SetVisibility (Variables|Character|GetMesh) false true)
    (Collision|SetCollisionResponsetoChannel (Variables|Default|GetCapsuleComponent) "ECC_Pawn" "ECR_Ignore")
    (bind _returnvalue (Effects|SpawnEmitterAttached "/Game/_Player/Dodge/P_FengMao_Dash_Trail_Mesh1.P_FengMao_Dash_Trail_Mesh1" (Variables|Character|GetMesh) "pelvis" "0, 0, 0" "0, 0, 0" "5.000000,5.000000,5.000000"))
    (Variables|Default|SetTeleportTrailEffect _returnvalue)
    (Effects|SpawnEmitteratLocation "/Game/_Player/Dodge/P_FengMao_Dash_Trail_Mesh1.P_FengMao_Dash_Trail_Mesh1" Location (Math|Rotator|FindLookatRotation (Transformation|GetActorLocation) Location) "5.000000,5.000000,5.000000")
    (Animation|StopAnimMontage 0)
    (Audio|PlaySoundatLocation "/Game/_Enemy/Boss/SFX/Boss_Teleport.Boss_Teleport" (Transformation|GetActorLocation) "0, 0, 0" 1.0 1.0 0.0 0 0 0 0)
    (AI|AIMoveTo self Location AttackTarget 1.5e+02 false
      (:OnSuccess
        _)
      (:OnFail
        _))
    (CallFunction|TeleportEnd)
    (else
      (Utilities|FlowControl|DelayUntilNextTick)
      (Default|CallOnTeleportEnd))))

(event Custom|TeleportEnd
  (bind _charactermovement (Variables|Character|GetCharacterMovement))
  ;[0 0.3458 1] Teleport
  (Components|Movement|StopMovementImmediately _charactermovement)
  (Pawn|Components|CharacterMovement|SetMovementMode _charactermovement "MOVE_Walking" 0)
  (Variables|/Script/Engine.CharacterMovementComponent|SetMaxAcceleration _charactermovement 1.5e+03)
  (Rendering|SetVisibility (Variables|Character|GetMesh) true true)
  (Collision|SetCollisionResponsetoChannel (Variables|Default|GetCapsuleComponent) "ECC_Pawn" "ECR_Block")
  (Default|CallOnTeleportEnd)
  (Utilities|FlowControl|Delay 0.5)
  (Variables|Default|SetisTeleporting false)
  (bind _teleporttraileffect (Variables|Default|GetTeleportTrailEffect)
    (:then
      (Components|DestroyComponent _teleporttraileffect))
    (:else)))

(event Custom|AttackCombo2
  (params (AttackTarget :type Actor%20Object%20Reference))
  ;[1 0 0] ATTACKS
  (CallFunction|Attack AttackTarget)
  (bind _notifyname (Animation|Montage|PlayMontage (Variables|Character|GetMesh) "/Game/_Enemy/Boss/NewAnimations/Attacks/BossSlamCombo_UE_Montage.BossSlamCombo_UE_Montage" 0.8)
    (:OnCompleted
      (CallFunction|AttackEnd AttackTarget :!label _label))
    (:OnInterrupted
      (goto _label))
    (:OnNotifyBegin
      (switch name _notifyname
        (:Slash
          (Default|SpehreTraceDamage (Variables|Default|GetBPC_Attacks) 4e+01 2.2e+02 (Utilities|Struct|MakeS_DamageInfo 15.0 "NewEnumerator1" "NewEnumerator1" false true true)))
        (:AOESlash
          (Default|AOESlash (Variables|Default|GetBPC_Attacks) (Utilities|Struct|MakeS_DamageInfo 2e+01 "NewEnumerator3" "NewEnumerator1" false false false true) 3e+02 AttackTarget))))))

(event Custom|ThrowAxe
  (params (AttackTarget :type Actor%20Object%20Reference))
  ;[1 0 0] ATTACKS
  (CallFunction|Attack AttackTarget)
  (bind _notifyname (Animation|Montage|PlayMontage (Variables|Character|GetMesh) "/Game/_Enemy/Boss/NewAnimations/Attacks/AxeThrow_UE_Montage.AxeThrow_UE_Montage" 1.5)
    (:OnCompleted
      (CallFunction|AttackEnd AttackTarget :!label _label)
      (Rendering|SetVisibility (Variables|/Game/_Enemy/Boss/Axe/BP_Axe.BP_Axe_C|GetStaticMesh (Variables|Default|GetAxe%20Ref)) true false))
    (:OnInterrupted
      (goto _label))
    (:OnNotifyBegin
      (switch name _notifyname
        (:Throw
          (Rendering|SetVisibility (Variables|/Game/_Enemy/Boss/Axe/BP_Axe.BP_Axe_C|GetStaticMesh (Variables|Default|GetAxe%20Ref)) false false)
          (bind _returnvalue (Game|SpawnActorfromClass "/Game/_Combat/Projectiles/BP_Projectile_Spinning_Axe.BP_Projectile_Spinning_Axe_C" (Math|Transform|MakeTransform (Transformation|GetSocketLocation (Variables|Character|GetMesh) "AxeSocket") "0, 0, 0" "2.000000,2.000000,2.000000") "Undefined" "MultiplyWithRoot" 0 4e+03 0.0 AttackTarget true self))
          (EventDispatchers|AssignOnProjectileImpact _returnvalue (delegate Custom|OnProjectileImpact_Event)))))))

(event Custom|OnProjectileImpact_Event
  (params (Other%20Actor :type Actor%20Object%20Reference) (Hit :type Hit%20Result%20Structure))
  ;[1 0 0] ATTACKS
  (Class|BPIDamagable|TakeDamage(Message) Other%20Actor (Utilities|Struct|MakeS_DamageInfo 2e+01 "NewEnumerator2" "NewEnumerator1" false false true) self))

(event Custom|QuickAttack
  (params (AttackTarget :type Actor%20Object%20Reference))
  ;[1 0 0] ATTACKS
  (Default|PrimaryMeleeAttack (Variables|Default|GetBPC_Attacks) (Utilities|Struct|MakeS_AttackInfo AttackTarget "/Game/_Enemy/Boss/NewAnimations/Attacks/BossFastSwing_UE_Montage.BossFastSwing_UE_Montage" (Utilities|Struct|MakeS_DamageInfo 2e+01 "NewEnumerator1" "NewEnumerator1" false true true)) 4e+01 2.2e+02))

(event Custom|JumpAttack
  (params (AttackTarget :type Actor%20Object%20Reference))
  ;[1 0 0] ATTACKS
  (Default|LongRangeMeleeAttack (Variables|Default|GetBPC_Attacks) (Utilities|Struct|MakeS_AttackInfo AttackTarget "/Game/_Enemy/Boss/NewAnimations/Attacks/BossJumpAttack_UE_Montage.BossJumpAttack_UE_Montage" (Utilities|Struct|MakeS_DamageInfo 2e+01 "NewEnumerator3" "NewEnumerator1" false false false true))))

(event EventBeginPlay
  (bind _bpc_damagesystem (Variables|Default|GetBPC_DamageSystem))
  (|CallParentFunction)
  (CallFunction|EquipWeapon)
  (UserInterface|SetWidget (Variables|Default|GetHealthbar) 0)
  (bind _returnvalue (UserInterface|CreateWidget "/Game/_UI/WB_BossHealthbar.WB_BossHealthbar_C"))
  (bind _output_get (Variables|Default|SetBossHealthbarREF _returnvalue))
  (Default|UpdateHealthPercentage _output_get (Variables|/Game/_Combat/BPC_DamageSystem.BPC_DamageSystem_C|GetHealth _bpc_damagesystem) (Variables|/Game/_Combat/BPC_DamageSystem.BPC_DamageSystem_C|GetMaxHealth _bpc_damagesystem))
  (bind _asbp_player (Utilities|Casting|CastToBP_Player (Game|Player|GetPlayerPawn 0)))
  (Variables|Default|SetPlayerREF _asbp_player))

(event Collision|EventActorBeginOverlap
  (params (OtherActor :type Actor%20Object%20Reference)))

(event EventTick
  (params (DeltaSeconds :type Float%20%28single-precision%29))
  (|CallParentFunction DeltaSeconds) ; This node is disabled and will not be called.\nDrag off pins to build functionality.
)

(event EventDeath
  (bind _returnvalue (Game|GetPlayerController 0))
  (bind _mesh (Variables|Character|GetMesh))
  ;[0 0 0] DEATH
  (Variables|/Game/_Combat/BPC_DamageSystem.BPC_DamageSystem_C|SetisDead (Variables|Default|GetBPC_DamageSystem) true)
  (Animation|StopAnimMontage 0)
  (Widget|RemovefromParent (Variables|Default|GetBossHealthbarREF))
  (Development|PrintString "Dead")
  (Collision|SetCollisionEnabled (Variables|Character|GetMesh) "QueryAndPhysics")
  (Rendering|SetVisibility (Variables|Default|GetHealthbar) false true)
  (AI|Logic|StopLogic (Variables|/Script/AIModule.AIController|GetBrainComponent (Variables|Default|GetAIC%20Enemy%20Base)) "")
  (Default|SetStateasDead (Variables|Default|GetAIC%20Enemy%20Base))
  (bind _keys (Utilities|Map|Keys (Variables|Default|GetReservedAttackTokens)))
  (for _array_element _keys
    (Class|BPIDamagable|ReturnAttackToken(Message) _array_element (.Value (Utilities|Map|Find (Variables|Default|GetReservedAttackTokens) _array_element)))
    (CallFunction|UnequipWeapon)
    (Animation|Montage|PlayMontage (Variables|Character|GetMesh) (Variables|Default|GetDeath%20Montage)
      (:then
        (bind _returnvalue_2 (UserInterface|CreateWidget "/Game/_UI/WB_BossDefeated.WB_BossDefeated_C" (Game|GetPlayerController 0)))
        (bind _output_get (Variables|Default|SetBossDefeatREF _returnvalue_2))
        (Class|VerticalBox|AddChildtoVerticalBox (Variables|/Game/_UI/PlerWidgets/W_Player_Healthbar.W_Player_Healthbar_C|GetCenterBox (Variables|/Game/_Player/BP_Player.BP_Player_C|GetHealthbarREF (Variables|Default|GetPlayerREF))) _output_get)
        (Utilities|FlowControl|Delay 2.0)
        (Widget|RemovefromParent (Variables|Default|GetBossDefeatREF))
        (Utilities|FlowControl|Delay 3.0)
        (bind _returnvalue_3 (UserInterface|CreateWidget "/Game/_UI/PlerWidgets/WB_GameOver.WB_GameOver_C"))
        (UserInterface|Viewport|AddtoViewport _returnvalue_3 0)
        (Game|SetGamePaused true)
        (Input|SetInputModeUIOnly _returnvalue _returnvalue_3 "DoNotLock" false)
        (Variables|/Script/Engine.PlayerController|SetbShowMouseCursor _returnvalue true)
        (Utilities|FlowControl|Delay 3.0)
        (Actor|DestroyActor))
      (:OnBlendOut
        (Collision|SetCollisionResponsetoAllChannels _mesh "ECR_Ignore")
        (Physics|SetSimulatePhysics _mesh true)))))

(fn ConstructionScript
  (bind _bpc_damagesystem (Variables|Default|GetBPC_DamageSystem))
  (|CallParentFunction)
  (bind _output_get (Variables|/Game/_Combat/BPC_DamageSystem.BPC_DamageSystem_C|SetMaxHealth _bpc_damagesystem 4e+02))
  (Variables|/Game/_Combat/BPC_DamageSystem.BPC_DamageSystem_C|SetHealth _bpc_damagesystem _output_get))

(fn SetMovementSpeed
  (params (Speed :type E_MovementSpeed%20Enum :default "NewEnumerator0"))
  (bind _output_get (Variables|/Script/Engine.CharacterMovementComponent|SetMaxWalkSpeed (Variables|Character|GetCharacterMovement) (Utilities|Select :Index Speed :NewEnumerator0 0.0 :NewEnumerator1 1e+02 :NewEnumerator2 2e+02 :NewEnumerator3 3.5e+02)))
  (return _output_get))

(fn TakeDamage
  (params (DamageInfo :type S%20Damage%20Info%20Structure) (DamageCauser :type Actor%20Object%20Reference))
  (bind _bpc_damagesystem (Variables|Default|GetBPC_DamageSystem))
  (bind _wasdamaged (|CallParentFunction DamageInfo DamageCauser))
  (Default|UpdateHealthPercentage (Variables|Default|GetBossHealthbarREF) (Variables|/Game/_Combat/BPC_DamageSystem.BPC_DamageSystem_C|GetHealth _bpc_damagesystem) (Variables|/Game/_Combat/BPC_DamageSystem.BPC_DamageSystem_C|GetMaxHealth _bpc_damagesystem))
  (return _wasdamaged))

(fn IsAttacking
  (bind _attacking (|CallParentFunction))
  (return _attacking))