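; BP_Sword is a sword actor that slices procedural meshes it passes through while the player's Slice flag is set.
; Begin overlap on SM_Sword captures the procedural mesh, and end overlap cuts it along a plane from the Point component's location and up vector.
; The cut creates a second half with a glowing cap, gives it physics and a fixed impulse, then destroys the overlapped actor after a delay.
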(event OnComponentBeginOverlap(SM_Sword)
  (params (OverlappedComponent :type Primitive%20Component%20Object%20Reference) (OtherActor :type Actor%20Object%20Reference) (OtherComp :type Primitive%20Component%20Object%20Reference) (OtherBodyIndex :type Integer) (bFromSweep :type Boolean) (SweepResult :type Hit%20Result%20Structure%20%28by%20ref%29))
  (if (Variables|/Game/_Player/BP_Player.BP_Player_C|GetSlice (Variables|Default|GetPLayerREF))
    (bind _asprocedural_mesh_component (Utilities|Casting|CastToProceduralMeshComponent OtherComp))))

(event OnComponentEndOverlap(SM_Sword)
  (params (OverlappedComponent :type Primitive%20Component%20Object%20Reference) (OtherActor :type Actor%20Object%20Reference) (OtherComp :type Primitive%20Component%20Object%20Reference) (OtherBodyIndex :type Integer))
  (bind _point (Variables|Default|GetPoint))
  (if (Variables|/Game/_Player/BP_Player.BP_Player_C|GetSlice (Variables|Default|GetPLayerREF))
    (Utilities|FlowControl|Sequence
      (:then_1
        (Utilities|IsValid (stale OnComponentBeginOverlap(SM_Sword) _asprocedural_mesh_component)
          (:Is%20Valid
            (bind _outotherhalfprocmesh (Class|KismetProceduralMeshLibrary|SliceProceduralMesh (stale OnComponentBeginOverlap(SM_Sword) _asprocedural_mesh_component) (Transformation|GetWorldLocation _point) (Math|Vector|GetUpVector _point) true "CreateNewSectionForCap" "/Game/Fracture/M_Glow_Inst.M_Glow_Inst"))
            (Physics|SetSimulatePhysics _outotherhalfprocmesh true)
            (Physics|AddImpulse _outotherhalfprocmesh "350.000000,350.000000,350.000000" "None" true)
            (Utilities|FlowControl|Delay 5.0)
            (Actor|DestroyActor (stale OnComponentBeginOverlap(SM_Sword) OtherActor))))))))

(event EventBeginPlay
  (bind _asbp_player (Utilities|Casting|CastToBP_Player (Game|Player|GetPlayerPawn 0)))
  (Variables|Default|SetPLayerREF _asbp_player))

(event Collision|EventActorBeginOverlap
  (params (OtherActor :type Actor%20Object%20Reference)))

(event EventTick
  (params (DeltaSeconds :type Float%20%28single-precision%29)))

(fn ConstructionScript)